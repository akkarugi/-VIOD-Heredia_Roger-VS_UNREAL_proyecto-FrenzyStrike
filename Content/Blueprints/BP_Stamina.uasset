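; BP_Stamina is a pickup actor that restores the player character's stamina.
; When an actor tagged Player overlaps its Sphere component, it plays a pickup sound and spawns a particle effect at its location.
; It then adds its Stamina value to the BP_ThirdPersonCharacter of player 0, with no clamp applied here, and destroys itself.
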(event `self.Sphere.OnComponentBeginOverlap`
  (params (OverlappedComponent :type "PrimitiveComponent Object Reference") (OtherActor :type "Actor Object Reference") (OtherComp :type "PrimitiveComponent Object Reference") (OtherBodyIndex :type Integer) (bFromSweep :type Boolean) (SweepResult :type "HitResult Structure (by ref)"))
  (bind _returnvalue (`self.K2_GetActorLocation`))
  (if (`self.ActorHasTag` OtherActor "Player")
    (`GameplayStatics.PlaySoundAtLocation` "/Engine/VREditor/Sounds/UI/Dockable_Window_Pick_Up.Dockable_Window_Pick_Up" _returnvalue (struct) 1.0 1.0 0.0 "/Game/Audio/SFX/SA_Character.SA_Character" null null null)
    (`GameplayStatics.SpawnEmitterAtLocation` "/Game/Realistic_Starter_VFX_Pack_Vol2/Particles/Destruction/P_Destruction_Metal.P_Destruction_Metal" _returnvalue (struct) (2.0 2.0 2.0) true "AutoRelease")
    (bind _asbp_third_person_character (cast `/Game/ThirdPerson/Blueprints/BP_ThirdPersonCharacter` (`GameplayStatics.GetPlayerCharacter` 0)))
    (set `/Game/ThirdPerson/Blueprints/BP_ThirdPersonCharacter.Stamina` (+ (`/Game/ThirdPerson/Blueprints/BP_ThirdPersonCharacter.Stamina` _asbp_third_person_character) (`self.+Stamina`)) _asbp_third_person_character)
    (`self.K2_DestroyActor`)))

(fn `UserConstructionScript`)