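; BP_Enemy2 is a melee enemy that chases the player once its PawnSensing component sees a pawn.
; AIMoveTo closes in, and on arrival it plays an attack montage with a whoosh sound, gated by CanAttack until the montage ends.
; A montage notify runs a forward sphere trace that damages and launches the player character, adding hit sound, particles and camera shake.
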(event `self.ReceiveBeginPlay`)

(event `ChasePlayer`
  (bind _returnvalue (`self.K2_GetActorLocation`))
  (`|AIMoveTo` self (0.0 0.0 0.0) (`GameplayStatics.GetPlayerCharacter` 0) 120.0
    (:`OnSuccess`
      (if (`self.canAttack?`)
        (`|PlayMontage` (`self.Mesh`) "/Game/Characters/Villager/Animations/Attack/A_Attack_Montage.A_Attack_Montage"
          (:`then`
            (set `self.canAttack?` false)
            (`GameplayStatics.PlaySoundAtLocation` "/Game/Audio/SFX/MS_AxeWhoosh.MS_AxeWhoosh" (`self.K2_GetActorLocation`) (struct) 1.0 1.0 0.0 null null null null))
          (:`OnCompleted`
            (set `self.canAttack?` true :!label _label))
          (:`OnInterrupted`
            (goto _label))
          (:`OnNotifyBegin`
            (bind (_outhit _returnvalue_2) (`KismetSystemLibrary.SphereTraceSingle` :`Start` _returnvalue :`End` (+ _returnvalue (* (`KismetMathLibrary.GetForwardVector` (`self.K2_GetActorRotation`)) 180.0)) :`Radius` 40.0 :`TraceChannel` "TraceTypeQuery3" :`bTraceComplex` true :`DrawTime` 0.5))
            (if _returnvalue_2
              (bind (_bblockinghit _binitialoverlap _time _distance _location _impactpoint _normal _impactnormal _physmat _hitactor) (`GameplayStatics.BreakHitResult` _outhit))
              (bind _asbp_third_person_character (cast `/Game/ThirdPerson/Blueprints/BP_ThirdPersonCharacter` _hitactor))
              (`/Game/ThirdPerson/Blueprints/BP_ThirdPersonCharacter.Take Damage` _asbp_third_person_character (`self.Damage`))
              (`self.LaunchCharacter` _asbp_third_person_character (+ (* (`KismetMathLibrary.GetForwardVector` (`self.K2_GetActorRotation`)) (`self.frontalKnockback`)) (`KismetMathLibrary.MakeVector` 0.0 0.0 (`self.upwardsKnockback`))) false false)
              (`GameplayStatics.PlaySoundAtLocation` "/Game/Audio/SFX/MS_AxeHit.MS_AxeHit" (`self.K2_GetActorLocation`) (struct) 1.0 1.0 0.0 null null null null)
              (`GameplayStatics.SpawnEmitterAtLocation` "/Game/Realistic_Starter_VFX_Pack_Vol2/Particles/Hit/P_Wood.P_Wood" _impactpoint (`KismetMathLibrary.MakeRotFromX` _normal) (1.5 1.5 1.5) true "AutoRelease")
              (`GameplayStatics.PlayWorldCameraShake` "/Game/Blueprints/BP_CameraShake_Hit.BP_CameraShake_Hit_C" _impactpoint 0.0 1000.0))))))))

(event `self.PawnSensing.OnSeePawn`
  (params (Pawn :type "Pawn Object Reference"))
  (`self.ChasePlayer`))

(fn `UserConstructionScript`)